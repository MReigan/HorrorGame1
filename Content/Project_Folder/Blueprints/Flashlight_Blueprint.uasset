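; Flashlight pickup actor that the first-person character collects by walking into it.
; An inner trigger box sets the character's PickedUp flag, plays a pickup sound and destroys the actor.
; A second box shows a widget component while the character overlaps it and hides it again when the overlap ends.
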(event OnComponentBeginOverlap(Box)
  (params (OverlappedComponent :type Primitive%20Component%20Object%20Reference) (OtherActor :type Actor%20Object%20Reference) (OtherComp :type Primitive%20Component%20Object%20Reference) (OtherBodyIndex :type Integer) (bFromSweep :type Boolean) (SweepResult :type Hit%20Result%20Structure%20%28by%20ref%29))
  (bind _asbp_first_person_character (Utilities|Casting|CastToBP_FirstPersonCharacter OtherActor))
  (Variables|/Game/Project_Folder/BP_FirstPersonCharacter.BP_FirstPersonCharacter_C|SetPicked%20Up _asbp_first_person_character true)
  (Audio|PlaySound2D "/Game/Project_Folder/Sounds/Picture_Pickup.Picture_Pickup" 1.0 1.0 0.0 0 0)
  (Actor|DestroyActor))

(event OnComponentBeginOverlap(Box_2)
  (params (OverlappedComponent :type Primitive%20Component%20Object%20Reference) (OtherActor :type Actor%20Object%20Reference) (OtherComp :type Primitive%20Component%20Object%20Reference) (OtherBodyIndex :type Integer) (bFromSweep :type Boolean) (SweepResult :type Hit%20Result%20Structure%20%28by%20ref%29))
  (Utilities|Casting|CastToBP_FirstPersonCharacter OtherActor)
  (Development|SetHiddeninGame (Variables|Default|GetWidget) false false))

(event OnComponentEndOverlap(Box_2)
  (params (OverlappedComponent :type Primitive%20Component%20Object%20Reference) (OtherActor :type Actor%20Object%20Reference) (OtherComp :type Primitive%20Component%20Object%20Reference) (OtherBodyIndex :type Integer))
  (Utilities|Casting|CastToBP_FirstPersonCharacter OtherActor)
  (Development|SetHiddeninGame (Variables|Default|GetWidget) true false))

(fn ConstructionScript)