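; Note_1 is an interactable note that opens and closes an on-screen note widget.
; Each Interact plays a paper sound and passes through a FlipFlop, with an IsOpen flag guarding both branches.
; Opening creates the widget, adds it to the viewport and sets the player controller to ignore look and move input.
; Closing calls PaperOut on the widget and restores that input.
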(event EventInteract
  (bind _returnvalue (Game|GetPlayerController 0))
  (Audio|PlaySound2D "/Game/Project_Folder/Sounds/Paper/Paper_Cue.Paper_Cue" 1.0 1.0 0.0 0 0)
  (Utilities|FlowControl|FlipFlop
    (:A
      (if (not (Variables|Default|GetIs%20Open))
        (bind _returnvalue_2 (Game|ConstructObjectfromClass "/Game/Project_Folder/Blueprints/Widgets/Notes/Note_1.Note_1_C"))
        (UserInterface|Viewport|AddtoViewport _returnvalue_2 0)
        (Input|SetIgnoreLookInput _returnvalue true)
        (Input|SetIgnoreMoveInput _returnvalue true)
        (Variables|Default|SetIs%20Open true)))
    (:B
      (if (Variables|Default|GetIs%20Open)
        (Default|PaperOut _returnvalue_2)
        (Input|SetIgnoreLookInput _returnvalue false)
        (Input|SetIgnoreMoveInput _returnvalue false)
        (Variables|Default|SetIs%20Open false)))))

(fn ConstructionScript)