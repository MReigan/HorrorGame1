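; Item inspection studio actor that shows a given mesh in a scene capture with a name and description widget while game time is frozen.
; Inspect moves input from the player to this actor, where mouse drag or movement axes rotate the item and the wheel adjusts capture FOV for zoom.
; Interaction closes the widget, destroys the actor, and either unfreezes time or returns focus to the inventory UI that opened it.
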(event EventInspect
  (params (Player :type BP%20First%20Person%20Character%20Object%20Reference) (Item%20To%20Focus :type Static%20Mesh%20Object%20Reference) (Item%20Name :type Text) (Item%20Description :type Text) (From%20UI :type Boolean) (UI :type Inventory%20Window%20Object%20Reference))
  (bind _returnvalue (Game|GetPlayerController 0))
  (Variables|Default|SetPlayer Player)
  (Components|StaticMesh|SetStaticMesh (Variables|Default|GetItem) Item%20To%20Focus)
  (Variables|Default|SetInventory UI)
  (Variables|Default|SetIs%20from%20UI From%20UI)
  (Audio|PlaySound2D (Variables|Default|GetSound) 1.0 1.0 0.0 0 0)
  (bind _returnvalue_2 (UserInterface|CreateWidget "/Game/Project_Folder/Blueprints/Widgets/Inspection_Widget.Inspection_Widget_C" 0 Item%20Name Item%20Description))
  (bind _output_get (Variables|Default|SetInspection%20Widget _returnvalue_2))
  (UserInterface|Viewport|AddtoViewport _output_get 0)
  (Input|DisableInput (Variables|Default|GetPlayer) _returnvalue)
  (Input|EnableInput _returnvalue)
  (Utilities|Time|SetGlobalTimeDilation 0.0))

(event Input|ActionEvents|InputActionInteraction
  (params (Key :type Key%20Structure :default "None"))
  (bind _returnvalue (Game|GetPlayerController 0))
  (bind _returnvalue_2 (Game|GetPlayerController 0))
  (:Pressed
    (if (Variables|Default|GetIs%20from%20UI)
      _
      (else
        (Utilities|Time|SetGlobalTimeDilation 1.0)))
    (Input|DisableInput _returnvalue_2)
    (Input|EnableInput (Variables|Default|GetPlayer) _returnvalue_2)
    (Widget|RemovefromParent (Variables|Default|GetInspection%20Widget))
    (Variables|Default|SetInspection%20Widget 0)
    (Actor|DestroyActor)
    (if (Variables|Default|GetIs%20from%20UI)
      (bind _inventory (Variables|Default|GetInventory)
        (:then
          (Input|SetInputModeUIOnly _returnvalue _inventory "DoNotLock" false)
          (Variables|/Script/Engine.PlayerController|SetbShowMouseCursor _returnvalue true))
        (:else)))))

(event Input|AxisEvents|InputAxisMoveForward/Backward
  (params (AxisValue :type Float%20%28single-precision%29))
  (if (!= AxisValue 0.0)
    (Transformation|SetWorldRotation (Variables|Default|GetItem) (Math|Rotator|CombineRotators (Transformation|GetWorldRotation (Variables|Default|GetItem)) (Math|Rotator|MakeRotator 0.0 (* AxisValue -1.0) 0.0)) false false)))

(event Input|AxisEvents|InputAxisMoveRight/Left
  (params (AxisValue :type Float%20%28single-precision%29))
  (if (!= AxisValue 0.0)
    (Transformation|SetWorldRotation (Variables|Default|GetItem) (Math|Rotator|CombineRotators (Transformation|GetWorldRotation (Variables|Default|GetItem)) (Math|Rotator|MakeRotator 0.0 0.0 (* AxisValue -1.0))) false false)))

(event Input|MouseEvents|MouseX
  (params (AxisValue :type Float%20%28single-precision%29))
  (if (Variables|Default|GetCan%20Rotate)
    (Transformation|SetWorldRotation (Variables|Default|GetItem) (Math|Rotator|CombineRotators (Transformation|GetWorldRotation (Variables|Default|GetItem)) (Math|Rotator|MakeRotator 0.0 0.0 (* AxisValue -2.0))) false false)))

(event Input|MouseEvents|MouseY
  (params (AxisValue :type Float%20%28single-precision%29))
  (if (Variables|Default|GetCan%20Rotate)
    (Transformation|SetWorldRotation (Variables|Default|GetItem) (Math|Rotator|CombineRotators (Transformation|GetWorldRotation (Variables|Default|GetItem)) (Math|Rotator|MakeRotator 0.0 (* AxisValue -2.0) 0.0)) false false)))

(event Input|MouseEvents|LeftMouseButton
  (params (Key :type Key%20Structure :default "None"))
  (:Pressed
    (Variables|Default|SetCan%20Rotate true))
  (:Released
    (Variables|Default|SetCan%20Rotate false)))

(event Input|MouseEvents|MouseWheelUp
  (params (Key :type Key%20Structure :default "None"))
  (bind _scenecapturecomponent2d (Variables|Default|GetSceneCaptureComponent2D))
  (:Pressed
    (Variables|/Script/Engine.SceneCaptureComponent2D|SetFOVAngle _scenecapturecomponent2d (Math|Float|Clamp(Float) (- (Variables|/Script/Engine.SceneCaptureComponent2D|GetFOVAngle _scenecapturecomponent2d) (Variables|Default|GetZoom%20Speed)) 3e+01 9e+01))))

(event Input|MouseEvents|MouseWheelDown
  (params (Key :type Key%20Structure :default "None"))
  (bind _scenecapturecomponent2d (Variables|Default|GetSceneCaptureComponent2D))
  (:Pressed
    (Variables|/Script/Engine.SceneCaptureComponent2D|SetFOVAngle _scenecapturecomponent2d (Math|Float|Clamp(Float) (+ (Variables|/Script/Engine.SceneCaptureComponent2D|GetFOVAngle _scenecapturecomponent2d) (Variables|Default|GetZoom%20Speed)) 3e+01 9e+01))))

(fn ConstructionScript)