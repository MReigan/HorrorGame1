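; Interactive elevator Blueprint that travels between two stops when the player presses E.
; Overlapping Box_3 enables the actor's input, and releasing E disables it again.
; The press plays a closed-door sound and eases the Elevator component between its relative origin and a lower offset over a fixed duration.
; An exact comparison against a hard-coded world height picks the direction, tying the logic to level placement.
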(event OnComponentBeginOverlap(Box_3)
  (params (OverlappedComponent :type Primitive%20Component%20Object%20Reference) (OtherActor :type Actor%20Object%20Reference) (OtherComp :type Primitive%20Component%20Object%20Reference) (OtherBodyIndex :type Integer) (bFromSweep :type Boolean) (SweepResult :type Hit%20Result%20Structure%20%28by%20ref%29))
  (Input|EnableInput (Game|GetPlayerController 0)))

(event Input|KeyboardEvents|E
  (params (Key :type Key%20Structure :default "None"))
  (:Pressed
    (if (== 2082.0 (.z (Transformation|GetWorldLocation (Variables|Default|GetElevator))))
      (Audio|SpawnSound2D "/Game/Project_Folder/Sounds/Closed_Door.Closed_Door" 1.0 1.0 0.0 0)
      (Components|MoveComponentTo (Variables|Default|GetElevator) "0.000000,0.000000,-1420.000000" "0, 0, 0" true true 8.0 false)
      (Utilities|FlowControl|Delay 8.0)
      (else
        (Audio|SpawnSound2D "/Game/Project_Folder/Sounds/Closed_Door.Closed_Door" 1.0 1.0 0.0 0)
        (Components|MoveComponentTo (Variables|Default|GetElevator) "0, 0, 0" "0, 0, 0" true true 8.0 false)
        (Utilities|FlowControl|Delay 8.0)))
    (Utilities|FlowControl|DoOnce false))
  (:Released
    (Input|DisableInput 0)
    (Utilities|FlowControl|DoOnce false)))

(fn ConstructionScript)