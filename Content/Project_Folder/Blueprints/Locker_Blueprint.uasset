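; Locker actor that the first-person player can hide in, with an animated door, sound and proximity widget.
; An overlap box enables input and opens a gate, so Interaction swings the door by timeline and calls ToggleHide.
; ToggleHide switches player movement, collision and visibility, blending the view between character and locker.
; While hiding, clamped mouse look drives the locker camera through a self-calling Delay loop in MoveCamera.
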(event OnComponentBeginOverlap(Box)
  (params (OverlappedComponent :type Primitive%20Component%20Object%20Reference) (OtherActor :type Actor%20Object%20Reference) (OtherComp :type Primitive%20Component%20Object%20Reference) (OtherBodyIndex :type Integer) (bFromSweep :type Boolean) (SweepResult :type Hit%20Result%20Structure%20%28by%20ref%29))
  (bind _asbp_first_person_character (Utilities|Casting|CastToBP_FirstPersonCharacter OtherActor))
  (bind _output_get (Variables|Default|SetCharacter_Reference _asbp_first_person_character))
  (Input|EnableInput (Game|GetPlayerController 0))
  (Utilities|FlowControl|Gate true) ; enters at Open
)

(event OnComponentEndOverlap(Box)
  (params (OverlappedComponent :type Primitive%20Component%20Object%20Reference) (OtherActor :type Actor%20Object%20Reference) (OtherComp :type Primitive%20Component%20Object%20Reference) (OtherBodyIndex :type Integer))
  (bind _returnvalue (Game|GetPlayerController 0))
  (bind _asbp_first_person_character (Utilities|Casting|CastToBP_FirstPersonCharacter OtherActor))
  (bind _output_get (Variables|Default|SetCharacter_Reference _asbp_first_person_character))
  (Input|DisableInput _returnvalue)
  (Utilities|FlowControl|Gate true) ; enters at Close
)

(event OnComponentBeginOverlap(WidgetBox)
  (params (OverlappedComponent :type Primitive%20Component%20Object%20Reference) (OtherActor :type Actor%20Object%20Reference) (OtherComp :type Primitive%20Component%20Object%20Reference) (OtherBodyIndex :type Integer) (bFromSweep :type Boolean) (SweepResult :type Hit%20Result%20Structure%20%28by%20ref%29))
  (Utilities|Casting|CastToBP_FirstPersonCharacter OtherActor)
  (Development|SetHiddeninGame (Variables|Default|GetWidget) false false))

(event OnComponentEndOverlap(WidgetBox)
  (params (OverlappedComponent :type Primitive%20Component%20Object%20Reference) (OtherActor :type Actor%20Object%20Reference) (OtherComp :type Primitive%20Component%20Object%20Reference) (OtherBodyIndex :type Integer))
  (Utilities|Casting|CastToBP_FirstPersonCharacter OtherActor)
  (Development|SetHiddeninGame (Variables|Default|GetWidget) true false))

(event Custom|Move%20Camera
  (if (Variables|Default|GetIs%20Hiding?)
    (Transformation|SetRelativeRotation (Variables|Default|GetCamera) (Math|Rotator|MakeRotator 0.0 (* (stale Input|AxisEvents|InputAxisLookUp/DownMouse _output_get) -1.0) (stale Input|AxisEvents|InputAxisTurnRight/LeftMouse _output_get)) false false)
    (Utilities|FlowControl|Delay 0.001)
    (CallFunction|MoveCamera)))

(event Custom|Hide
  (Rendering|SetActorHiddenInGame (stale OnComponentBeginOverlap(Box) _output_get) true))

(event Custom|Unhide
  (Rendering|SetActorHiddenInGame (stale OnComponentEndOverlap(Box) _output_get) false))

(event Input|ActionEvents|InputActionInteraction
  (params (Key :type Key%20Structure :default "None"))
  (:Pressed
    (Utilities|FlowControl|DoOnce false :!label _label
      (:Completed
        (Audio|PlaySound2D "/Game/Project_Folder/Sounds/Locker.Locker" 1.0 1.0 0.0 0 0)
        (Utilities|FlowControl|Gate true :!label _label_2
          (:Exit
            (Utilities|FlowControl|Sequence
              (:then_0
                (CallFunction|ToggleHide)
                (CallFunction|MoveCamera)
                (Utilities|FlowControl|Delay 0.2)
                (Input|EnableInput (Game|GetPlayerController 0))
                (goto _label_2 Open))
              (:then_1
                (bind _door_track (Timeline|Open%20And%20Close%20Door PlayFromStart)
                  (:Update
                    (Transformation|SetRelativeRotation (Variables|Default|GetScene) (Math|Rotator|MakeRotator 0.0 0.0 (Math|Float|Lerp (Variables|Default|GetClose%20Angle) (Variables|Default|GetOpen%20Angle) _door_track)) false false))
                  (:Finished
                    (goto _label Reset)))))))))))

(event Input|AxisEvents|InputAxisLookUp/DownMouse
  (params (AxisValue :type Float%20%28single-precision%29))
  (if (Variables|Default|GetIs%20Hiding?)
    (bind _output_get (Variables|Default|SetPitch (Math|Float|Clamp(Float) (+ (Variables|Default|GetPitch) AxisValue) -1e+01 2e+01)))
    (else
      (Pawn|Input|AddControllerPitchInput (Variables|Default|GetCharacter_Reference) AxisValue))))

(event Input|AxisEvents|InputAxisTurnRight/LeftMouse
  (params (AxisValue :type Float%20%28single-precision%29))
  (if (Variables|Default|GetIs%20Hiding?)
    (bind _output_get (Variables|Default|SetYaw (Math|Float|Clamp(Float) (+ (Variables|Default|GetYaw) AxisValue) -3e+01 3e+01)))
    (else
      (Pawn|Input|AddControllerYawInput (Variables|Default|GetCharacter_Reference) 0.0))))

(fn ConstructionScript)

(fn ToggleHide
  (bind _returnvalue (Game|GetPlayerController 0))
  (bind _character_reference (Variables|Default|GetCharacter_Reference))
  (bind _charactermovement (Variables|/Script/Engine.Character|GetCharacterMovement _character_reference))
  (if (Variables|Default|GetIs%20Hiding?)
    (Variables|Default|SetIs%20Hiding? false)
    (Pawn|Components|CharacterMovement|SetMovementMode _charactermovement "MOVE_Walking" 0)
    (Utilities|Time|SetTimerbyFunctionName 0 "Unhide" 1.0)
    (Collision|SetActorEnableCollision _character_reference true)
    (Game|Player|SetViewTargetwithBlend _returnvalue _character_reference 1.0 "VTBlend_Linear" 0.0 false)
    (else
      (Variables|Default|SetIs%20Hiding? true)
      (Pawn|Components|CharacterMovement|SetMovementMode _charactermovement "MOVE_None" 0)
      (Utilities|Time|SetTimerbyFunctionName 0 "Hide" 0.1)
      (Collision|SetActorEnableCollision _character_reference false)
      (Game|Player|SetViewTargetwithBlend _returnvalue self 1.0 "VTBlend_Linear" 0.0 false))))