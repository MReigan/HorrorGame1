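; Inventory component that holds a fixed number of item slots and opens or closes their inventory window.
; Adding an item tops up the first partial stack of the same class or fills the first empty slot, recursing on overflow past the max stack size.
; Toggling creates or removes the window on the first-person character's HUD canvas, switching input mode and cursor visibility with sound cues.
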(event EventBeginPlay
  (Utilities|Array|Resize (Variables|Default|GetInventory) (Variables|Default|GetNumber%20Of%20Slots)))

(fn ToggleInventory
  (bind _returnvalue (Game|GetPlayerController 0))
  (bind _returnvalue_2 (Game|GetPlayerController 0))
  (Audio|PlaySound2D 0 1.0 1.0 0.0 0 0)
  (Variables|Default|GetInventory%20UI
    (:then
      (bind _asinventory_slot (Utilities|Casting|CastToInventory_Slot (Class|PanelWidget|GetChildat (Variables|/Game/Project_Folder/Blueprints/Inventory_System/UI/Inventory_Window.Inventory_Window_C|GetInventoryGrid (Variables|Default|GetInventory%20UI)))))
      (Default|DisableActionBar _asinventory_slot)
      (Utilities|Time|SetGlobalTimeDilation 1.0)
      (Audio|PlaySound2D "/Game/Project_Folder/Sounds/Inventory_Close.Inventory_Close" 1.0 1.0 0.0 0 0)
      (Widget|RemovefromParent (Variables|Default|GetInventory%20UI))
      (Variables|Default|SetInventory%20UI 0)
      (Input|SetInputModeGameOnly _returnvalue false)
      (Variables|/Script/Engine.PlayerController|SetbShowMouseCursor _returnvalue false))
    (:else
      (Utilities|Time|SetGlobalTimeDilation 1.0)
      (Audio|PlaySound2D "/Game/Project_Folder/Sounds/Description_Item.Description_Item" 1.0 1.0 0.0 0 0)
      (bind _returnvalue_3 (UserInterface|CreateWidget "/Game/Project_Folder/Blueprints/Inventory_System/UI/Inventory_Window.Inventory_Window_C" 0 self (Variables|Default|GetName)))
      (bind _output_get (Variables|Default|SetInventory%20UI _returnvalue_3))
      (bind _asbp_first_person_character (Utilities|Casting|CastToBP_FirstPersonCharacter (Game|GetPlayerCharacter 0)))
      (bind _returnvalue_4 (Class|CanvasPanel|AddChildtoCanvas (Variables|/Game/Project_Folder/Blueprints/Inventory_System/Hud.Hud_C|GetCanvas (Variables|/Game/Project_Folder/BP_FirstPersonCharacter.BP_FirstPersonCharacter_C|GetHud _asbp_first_person_character)) _output_get))
      (Class|CanvasPanelSlot|SetAutoSize _returnvalue_4 true)
      (Class|CanvasPanelSlot|SetAlignment _returnvalue_4 "(X=0.500000,Y=7.000000)")
      (Class|CanvasPanelSlot|SetAnchors _returnvalue_4 (Utilities|Struct|MakeAnchors "(X=0.700000,Y=0.070000)" "(X=1.000000,Y=1.000000)"))
      (Input|SetInputModeUIOnly _returnvalue_2 _output_get "DoNotLock" false)
      (Variables|/Script/Engine.PlayerController|SetbShowMouseCursor _returnvalue_2 true))))

(fn AddtoInventory
  (params (Items%20To%20Add :type Slot%20Structure%20Structure))
  (if (.isstackable (.ItemStructure (Utilities|Struct|BreakSlot_Structure Items%20To%20Add)))
    (bind _slot_index (Utilities|HasPartialStack Items%20To%20Add)
      (:True
        (bind _success (CallFunction|AddtoStack Items%20To%20Add _slot_index))
        (LocalVariables|SetIs%20Success _success))
      (:False
        (bind _success_2 (CallFunction|CreateStack Items%20To%20Add :!label _label))
        (LocalVariables|SetIs%20Success _success_2)))
    (else
      (goto _label)))
  (return (LocalVariables|GetIs%20Success)))

(fn CreateStack
  (params (Slot :type Slot%20Structure%20Structure))
  (bind (_array_element _array_index) (Utilities|Array|ForEachLoopwithBreak (Variables|Default|GetInventory) :!label _label)
    (:LoopBody
      (if (<= (.quantity _array_element) 0)
        (LocalVariables|SetHas%20Space true)
        (LocalVariables|SetEmpty%20Index _array_index)
        (goto _label Break)))
    (:Completed
      (if (LocalVariables|GetHas%20Space)
        (Utilities|Array|SetArrayElem (Variables|Default|GetInventory) (LocalVariables|GetEmpty%20Index) Slot)
        (return (LocalVariables|GetHas%20Space))
        (else
          (return false))))))

(fn AddtoStack
  (params (Slot :type Slot%20Structure%20Structure) (Index :type Integer))
  (bind _inventory (Variables|Default|GetInventory))
  (bind _inventory_2 (Variables|Default|GetInventory))
  (bind _maxstacksize (Utilities|Struct|BreakItem_Structure (.itemstructure Slot)))
  (bind _output (Utilities|Array|Get(acopy) _inventory Index))
  (bind _output_2 (Utilities|Array|Get(acopy) _inventory_2 Index))
  (bind _output_get (LocalVariables|SetCurrent%20Quantity (.quantity _output)))
  (if (> (+ _output_get (.Quantity (Utilities|Struct|BreakSlot_Structure Slot))) (.maxstacksize (.itemstructure _output)))
    (Utilities|Array|SetArrayElem (Variables|Default|GetInventory) Index (Utilities|Struct|MakeSlot_Structure (.itemstructure Slot) _maxstacksize))
    (CallFunction|AddtoInventory (Utilities|Struct|MakeSlot_Structure "(ItemName_43_A0597D61427748DD6A903AB5AFDB84C8=\"\",ItemDescription_44_1204DB1D48BF2FC9CA97ED8B14798106=\"\",CanBeAdded?_7_9A7013F14F5FE936FAF240822D7C295B=False,ItemIcon_10_4E1D5F2A42B7E0525168B2B457D59320=None,IsStackable_13_EF50689E481C5D35708BCBB051867848=False,IsPickUpBenefitial_16_C6A420CF41A7163041834F9C13210411=False,ItemClass_20_B7BED92D44E23CA9619F5A8A418AB8DA=None,MaxStackSize_23_0CCB14BE4139813C23F326A12CB7C1D6=0,Staticmesh_27_F6C305A5428921ED26D2338FD9E7AA68=None,CanCombine?_29_D8229E7D49530A369A4164AB8432DDF8=False,Combination_35_FC72F94748621460FA63438AA25B4E9F=(),CanDiscard?_38_739AD3B645388BAB65714EB5E21BC4FF=False,IsUsable_40_F143D90845786F95685FC59C503C8830=False)" (- (.quantity Slot) (- _maxstacksize (LocalVariables|GetCurrent%20Quantity)))))
    (else
      (Utilities|Array|SetArrayElem _inventory_2 Index (Utilities|Struct|MakeSlot_Structure (.itemstructure _output_2) (+ (.quantity _output_2) (.quantity Slot))))))
  (return true))