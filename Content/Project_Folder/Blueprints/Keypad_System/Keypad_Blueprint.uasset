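; Interactive keypad actor where the player enters a code to trigger a success message on a target.
; Collision overlap registers it with the first-person character; interacting locks movement, blends to the keypad camera and enables mouse clicks.
; Child-actor buttons receive a keypad reference, and entries edit the displayed text.
; Confirming compares it with the code: success restores player control, removes collision and notifies the target, while failure re-initialises entry after a delay.
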(event OnComponentBeginOverlap(CollisionBox)
  (params (OverlappedComponent :type Primitive%20Component%20Object%20Reference) (OtherActor :type Actor%20Object%20Reference) (OtherComp :type Primitive%20Component%20Object%20Reference) (OtherBodyIndex :type Integer) (bFromSweep :type Boolean) (SweepResult :type Hit%20Result%20Structure%20%28by%20ref%29))
  (if (== OtherActor (Game|Player|GetPlayerPawn 0))
    (bind _asbp_first_person_character (Utilities|Casting|CastToBP_FirstPersonCharacter OtherActor))
    (Variables|/Game/Project_Folder/BP_FirstPersonCharacter.BP_FirstPersonCharacter_C|SetKeypad%20Interact _asbp_first_person_character self)
    (Variables|Default|SetPlayer%20Reference _asbp_first_person_character)))

(event OnComponentEndOverlap(CollisionBox)
  (params (OverlappedComponent :type Primitive%20Component%20Object%20Reference) (OtherActor :type Actor%20Object%20Reference) (OtherComp :type Primitive%20Component%20Object%20Reference) (OtherBodyIndex :type Integer))
  (if (== OtherActor (Game|Player|GetPlayerPawn 0))
    (bind _asbp_first_person_character (Utilities|Casting|CastToBP_FirstPersonCharacter OtherActor))
    (Variables|/Game/Project_Folder/BP_FirstPersonCharacter.BP_FirstPersonCharacter_C|SetKeypad%20Interact _asbp_first_person_character 0)
    (Variables|Default|SetPlayer%20Reference 0)))

(event Custom|Initiate
  (bind _returnvalue (Game|GetPlayerController 0))
  (bind _self self)
  (bind _text_code (Variables|Default|GetText%20Code))
  (bind _output_get (Variables|/Script/Engine.PlayerController|SetbShowMouseCursor _returnvalue true))
  (bind _output_get_2 (Variables|/Script/Engine.PlayerController|SetbEnableClickEvents _returnvalue _output_get))
  (Variables|/Script/Engine.PlayerController|SetbEnableMouseOverEvents _returnvalue _output_get_2)
  (Rendering|Components|TextRender|SetText _text_code (Utilities|Text|MakeLiteralText (Utilities|Text|ToText(String) (Utilities|String|GetSubstring (Utilities|String|MakeLiteralString) 0 (Utilities|String|Len (Variables|Default|GetKeypad_Code))))))
  (Rendering|Components|TextRender|SetTextRenderColor _text_code (Math|Color|MakeColor 200 200 200 255))
  (bind _output_get_3 (Variables|Default|SetButton_Array (Utilities|Array|MakeArray (Variables|Default|GetKeypad_Buttons_0) (Variables|Default|GetKeypad_Buttons_1) (Variables|Default|GetKeypad_Buttons_2) (Variables|Default|GetKeypad_Buttons_3) (Variables|Default|GetKeypad_Buttons_4) (Variables|Default|GetKeypad_Buttons_5) (Variables|Default|GetKeypad_Buttons_6) (Variables|Default|GetKeypad_Buttons_7) (Variables|Default|GetKeypad_Buttons_8) (Variables|Default|GetKeypad_Buttons_9) (Variables|Default|GetKeypad_Buttons_Backspace) (Variables|Default|GetKeypad_Buttons_Enter))))
  (for _array_element _output_get_3
    (Utilities|FlowControl|Sequence
      (:then_0
        (bind _askeypad_button_2_blueprint (Utilities|Casting|CastToKeypad_Button_2_Blueprint (Variables|/Script/Engine.ChildActorComponent|GetChildActor _array_element)))
        (Variables|/Game/Project_Folder/Blueprints/Keypad_System/Buttons/Keypad_Button_2_Blueprint.Keypad_Button_2_Blueprint_C|SetKeypad%20Actor%20Reference _askeypad_button_2_blueprint _self))
      (:then_1
        (bind _askeypad_button_1_blueprint (Utilities|Casting|CastToKeypad_Button_1_Blueprint (Variables|/Script/Engine.ChildActorComponent|GetChildActor _array_element)))
        (Variables|/Game/Project_Folder/Blueprints/Keypad_System/Buttons/Keypad_Button_1_Blueprint.Keypad_Button_1_Blueprint_C|SetKeypad%20Actor%20Reference _askeypad_button_1_blueprint _self))
      (:then_2
        (bind _askeypad_button_backspace_blueprint (Utilities|Casting|CastToKeypad_Button_Backspace_Blueprint (Variables|/Script/Engine.ChildActorComponent|GetChildActor _array_element)))
        (Variables|/Game/Project_Folder/Blueprints/Keypad_System/Buttons/Keypad_Button_Backspace_Blueprint.Keypad_Button_Backspace_Blueprint_C|SetKeypad%20Actor%20Reference _askeypad_button_backspace_blueprint _self))
      (:then_3
        (bind _askeypad_button_3_blueprint (Utilities|Casting|CastToKeypad_Button_3_Blueprint (Variables|/Script/Engine.ChildActorComponent|GetChildActor _array_element)))
        (Variables|/Game/Project_Folder/Blueprints/Keypad_System/Buttons/Keypad_Button_3_Blueprint.Keypad_Button_3_Blueprint_C|SetKeypad%20Actor%20Reference _askeypad_button_3_blueprint _self))
      (:then_4
        (bind _askeypad_button_4_blueprint (Utilities|Casting|CastToKeypad_Button_4_Blueprint (Variables|/Script/Engine.ChildActorComponent|GetChildActor _array_element)))
        (Variables|/Game/Project_Folder/Blueprints/Keypad_System/Buttons/Keypad_Button_4_Blueprint.Keypad_Button_4_Blueprint_C|SetKeypad%20Actor%20Reference _askeypad_button_4_blueprint _self))
      (:then_5
        (bind _askeypad_button_5_blueprint (Utilities|Casting|CastToKeypad_Button_5_Blueprint (Variables|/Script/Engine.ChildActorComponent|GetChildActor _array_element)))
        (Variables|/Game/Project_Folder/Blueprints/Keypad_System/Buttons/Keypad_Button_5_Blueprint.Keypad_Button_5_Blueprint_C|SetKeypad%20Actor%20Reference _askeypad_button_5_blueprint _self))
      (:then_6
        (bind _askeypad_button_6_blueprint (Utilities|Casting|CastToKeypad_Button_6_Blueprint (Variables|/Script/Engine.ChildActorComponent|GetChildActor _array_element)))
        (Variables|/Game/Project_Folder/Blueprints/Keypad_System/Buttons/Keypad_Button_6_Blueprint.Keypad_Button_6_Blueprint_C|SetKeypad%20Actor%20Reference _askeypad_button_6_blueprint _self))
      (:then_7
        (bind _askeypad_button_7_blueprint (Utilities|Casting|CastToKeypad_Button_7_Blueprint (Variables|/Script/Engine.ChildActorComponent|GetChildActor _array_element)))
        (Variables|/Game/Project_Folder/Blueprints/Keypad_System/Buttons/Keypad_Button_7_Blueprint.Keypad_Button_7_Blueprint_C|SetKeypad%20Actor%20Reference _askeypad_button_7_blueprint _self))
      (:then_8
        (bind _askeypad_button_8_blueprint (Utilities|Casting|CastToKeypad_Button_8_Blueprint (Variables|/Script/Engine.ChildActorComponent|GetChildActor _array_element)))
        (Variables|/Game/Project_Folder/Blueprints/Keypad_System/Buttons/Keypad_Button_8_Blueprint.Keypad_Button_8_Blueprint_C|SetKeypad%20Actor%20Reference _askeypad_button_8_blueprint _self))
      (:then_9
        (bind _askeypad_button_9_blueprint (Utilities|Casting|CastToKeypad_Button_9_Blueprint (Variables|/Script/Engine.ChildActorComponent|GetChildActor _array_element)))
        (Variables|/Game/Project_Folder/Blueprints/Keypad_System/Buttons/Keypad_Button_9_Blueprint.Keypad_Button_9_Blueprint_C|SetKeypad%20Actor%20Reference _askeypad_button_9_blueprint _self))
      (:then_10
        (bind _askeypad_button_enter_blueprint (Utilities|Casting|CastToKeypad_Button_Enter_Blueprint (Variables|/Script/Engine.ChildActorComponent|GetChildActor _array_element)))
        (Variables|/Game/Project_Folder/Blueprints/Keypad_System/Buttons/Keypad_Button_Enter_Blueprint.Keypad_Button_Enter_Blueprint_C|SetKeypad%20Actor%20Reference _askeypad_button_enter_blueprint _self))
      (:then_11
        (bind _askeypad_button_0_blueprint (Utilities|Casting|CastToKeypad_Button_0_Blueprint (Variables|/Script/Engine.ChildActorComponent|GetChildActor _array_element)))
        (Variables|/Game/Project_Folder/Blueprints/Keypad_System/Buttons/Keypad_Button_0_Blueprint.Keypad_Button_0_Blueprint_C|SetKeypad%20Actor%20Reference _askeypad_button_0_blueprint _self)))))

(event Custom|Button%20Entered
  (params (Value :type Text) (Confirmed :type Boolean) (Backspace :type Boolean))
  (bind _text_code (Variables|Default|GetText%20Code))
  (if Confirmed
    (CallFunction|OnConfirmed)
    (elif Backspace
      (CallFunction|Backspace)
      (elif (Variables|Default|GetCan_Enter)
        (Audio|PlaySound2D "/Game/Project_Folder/Sounds/Enter_Button.Enter_Button" 1.0 1.0 0.0 0 0)
        (Rendering|Components|TextRender|SetText _text_code (Utilities|Text|ToText(String) (Utilities|String|Replace (Utilities|String|ToString(Text) (Variables|/Script/Engine.TextRenderComponent|GetText (Variables|Default|GetText%20Code))) (Utilities|String|GetSubstring (Utilities|String|MakeLiteralString) 0 (Utilities|String|Len (Variables|Default|GetKeypad_Code))))))
        (Rendering|Components|TextRender|SetText _text_code (Utilities|Text|ToText(String) (Utilities|String|Append (Utilities|String|ToString(Text) (Variables|/Script/Engine.TextRenderComponent|GetText (Variables|Default|GetText%20Code))) (Utilities|String|ToString(Text) Value))))
        (Rendering|Components|TextRender|SetTextRenderColor (Variables|Default|GetText%20Code) (Math|Color|MakeColor 255 255 255 255))))))

(event Custom|Backspace
  (bind _text_code (Variables|Default|GetText%20Code))
  (bind _text (Variables|/Script/Engine.TextRenderComponent|GetText _text_code))
  (bind _returnvalue (Utilities|String|ToString(Text) _text))
  (Audio|PlaySound2D "/Game/Project_Folder/Sounds/Enter_Button.Enter_Button" 1.0 1.0 0.0 0 0)
  (Rendering|Components|TextRender|SetText _text_code (Utilities|Text|ToText(String) (Utilities|String|GetSubstring _returnvalue 0 (- (Utilities|String|Len _returnvalue) 1)))))

(event Custom|On%20Confirmed
  (bind _returnvalue (Game|GetPlayerController 0))
  (bind _returnvalue_2 (Game|GetPlayerController 0))
  (bind _returnvalue_3 (Game|GetPlayerController 0))
  (if (Utilities|Enum|Equal(Enum) (Variables|Default|GetKeypad_Code) (Utilities|String|ToString(Text) (Variables|/Script/Engine.TextRenderComponent|GetText (Variables|Default|GetText%20Code))))
    (Utilities|FlowControl|Sequence
      (:then_0
        (Rendering|Components|TextRender|SetTextRenderColor (Variables|Default|GetText%20Code) (Math|Color|MakeColor 0 255 0 255))
        (Rendering|Material|SetMaterial (Variables|Default|GetKeypad) 1 "/Game/Project_Folder/Blueprints/Keypad_System/Textures/Green_Light/Green_Light.Green_Light")
        (Utilities|FlowControl|RetriggerableDelay 2.0)
        (bind _output_get (Variables|/Script/Engine.PlayerController|SetbShowMouseCursor _returnvalue_2 false))
        (bind _output_get_2 (Variables|/Script/Engine.PlayerController|SetbEnableMouseOverEvents _returnvalue_2 _output_get))
        (Variables|/Script/Engine.PlayerController|SetbEnableClickEvents _returnvalue_2 _output_get_2)
        (for _array_element (Variables|Default|GetButton_Array)
          (bind _askeypad_button_1_blueprint (Utilities|Casting|CastToKeypad_Button_1_Blueprint (Variables|/Script/Engine.ChildActorComponent|GetChildActor _array_element)))
          (Default|ResetButtons _askeypad_button_1_blueprint))
        (Game|Player|SetViewTargetwithBlend (Game|GetPlayerController 0) (Components|GetOwner (Variables|/Game/Project_Folder/BP_FirstPersonCharacter.BP_FirstPersonCharacter_C|GetFirstPersonCamera (.AsBP%20First%20Person%20Character (Utilities|Casting|CastToBP_FirstPersonCharacter (Game|Player|GetPlayerPawn 0))))) 0.5 "VTBlend_Linear" 0.0 false)
        (Rendering|Components|TextRender|SetText (Variables|Default|GetText%20Code) (Utilities|Text|MakeLiteralText ""))
        (Input|SetInputModeGameOnly _returnvalue_3 false)
        (Components|DestroyComponent (Variables|Default|GetCollision%20Box))
        (Input|SetIgnoreMoveInput _returnvalue_3 false)
        (Class|KeypadSuccesInterface|OnSuccess(Message) (Variables|Default|GetKeypad_Target)))
      (:then_1
        (Variables|Default|SetCan_Enter false)
        (Audio|PlaySound2D "/Game/Project_Folder/Sounds/Enter_Button.Enter_Button" 1.0 1.0 0.0 0 0)
        (Audio|PlaySound2D "/Game/Project_Folder/Sounds/Success_Button.Success_Button" 1.0 1.0 0.0 0 0)))
    (else
      (Utilities|FlowControl|Sequence
        (:then_0
          (Rendering|Components|TextRender|SetTextRenderColor (Variables|Default|GetText%20Code) (Math|Color|MakeColor 0 0 255 255))
          (Rendering|Material|SetMaterial (Variables|Default|GetKeypad) 1 "/Game/Project_Folder/Blueprints/Keypad_System/Keypad_Material.Keypad_Material")
          (Utilities|FlowControl|RetriggerableDelay 2.0)
          (bind _output_get_3 (Variables|/Script/Engine.PlayerController|SetbEnableMouseOverEvents _returnvalue false))
          (Variables|/Script/Engine.PlayerController|SetbEnableClickEvents _returnvalue _output_get_3)
          (for _array_element_2 (Variables|Default|GetButton_Array)
            (bind _askeypad_button_1_blueprint_2 (Utilities|Casting|CastToKeypad_Button_1_Blueprint (Variables|/Script/Engine.ChildActorComponent|GetChildActor _array_element_2)))
            (Default|ResetButtons _askeypad_button_1_blueprint_2))
          (CallFunction|Initiate)
          (Variables|Default|SetCan_Enter true))
        (:then_1
          (Variables|Default|SetCan_Enter false)
          (Audio|PlaySound2D "/Game/Project_Folder/Sounds/Flashlight_On.Flashlight_On" 1.0 1.0 0.0 0 0))))))

(event Custom|On%20Interacted
  (bind _returnvalue (Game|GetPlayerController 0))
  (bind _returnvalue_2 (Game|GetPlayerController 0))
  (bind _self self)
  (bind _text_code (Variables|Default|GetText%20Code))
  (Input|SetIgnoreMoveInput _returnvalue true)
  (Game|Player|SetViewTargetwithBlend _returnvalue (Components|GetOwner (Variables|Default|GetCamera)) 0.4 "VTBlend_Linear" 0.0 false)
  (bind _output_get (Variables|/Script/Engine.PlayerController|SetbShowMouseCursor _returnvalue_2 true))
  (bind _output_get_2 (Variables|/Script/Engine.PlayerController|SetbEnableClickEvents _returnvalue_2 _output_get))
  (Variables|/Script/Engine.PlayerController|SetbEnableMouseOverEvents _returnvalue_2 _output_get_2)
  (Rendering|Components|TextRender|SetText _text_code (Utilities|Text|MakeLiteralText (Utilities|Text|ToText(String) (Utilities|String|GetSubstring (Utilities|String|MakeLiteralString) 0 (Utilities|String|Len (Variables|Default|GetKeypad_Code))))))
  (Rendering|Components|TextRender|SetTextRenderColor _text_code (Math|Color|MakeColor 200 200 200 255))
  (bind _output_get_3 (Variables|Default|SetButton_Array (Utilities|Array|MakeArray (Variables|Default|GetKeypad_Buttons_0) (Variables|Default|GetKeypad_Buttons_1) (Variables|Default|GetKeypad_Buttons_2) (Variables|Default|GetKeypad_Buttons_3) (Variables|Default|GetKeypad_Buttons_4) (Variables|Default|GetKeypad_Buttons_5) (Variables|Default|GetKeypad_Buttons_6) (Variables|Default|GetKeypad_Buttons_7) (Variables|Default|GetKeypad_Buttons_8) (Variables|Default|GetKeypad_Buttons_9) (Variables|Default|GetKeypad_Buttons_Backspace) (Variables|Default|GetKeypad_Buttons_Enter))))
  (for _array_element _output_get_3
    (Utilities|FlowControl|Sequence
      (:then_0
        (bind _askeypad_button_2_blueprint (Utilities|Casting|CastToKeypad_Button_2_Blueprint (Variables|/Script/Engine.ChildActorComponent|GetChildActor _array_element)))
        (Variables|/Game/Project_Folder/Blueprints/Keypad_System/Buttons/Keypad_Button_2_Blueprint.Keypad_Button_2_Blueprint_C|SetKeypad%20Actor%20Reference _askeypad_button_2_blueprint _self))
      (:then_1
        (bind _askeypad_button_1_blueprint (Utilities|Casting|CastToKeypad_Button_1_Blueprint (Variables|/Script/Engine.ChildActorComponent|GetChildActor _array_element)))
        (Variables|/Game/Project_Folder/Blueprints/Keypad_System/Buttons/Keypad_Button_1_Blueprint.Keypad_Button_1_Blueprint_C|SetKeypad%20Actor%20Reference _askeypad_button_1_blueprint _self))
      (:then_2
        (bind _askeypad_button_backspace_blueprint (Utilities|Casting|CastToKeypad_Button_Backspace_Blueprint (Variables|/Script/Engine.ChildActorComponent|GetChildActor _array_element)))
        (Variables|/Game/Project_Folder/Blueprints/Keypad_System/Buttons/Keypad_Button_Backspace_Blueprint.Keypad_Button_Backspace_Blueprint_C|SetKeypad%20Actor%20Reference _askeypad_button_backspace_blueprint _self))
      (:then_3
        (bind _askeypad_button_3_blueprint (Utilities|Casting|CastToKeypad_Button_3_Blueprint (Variables|/Script/Engine.ChildActorComponent|GetChildActor _array_element)))
        (Variables|/Game/Project_Folder/Blueprints/Keypad_System/Buttons/Keypad_Button_3_Blueprint.Keypad_Button_3_Blueprint_C|SetKeypad%20Actor%20Reference _askeypad_button_3_blueprint _self))
      (:then_4
        (bind _askeypad_button_4_blueprint (Utilities|Casting|CastToKeypad_Button_4_Blueprint (Variables|/Script/Engine.ChildActorComponent|GetChildActor _array_element)))
        (Variables|/Game/Project_Folder/Blueprints/Keypad_System/Buttons/Keypad_Button_4_Blueprint.Keypad_Button_4_Blueprint_C|SetKeypad%20Actor%20Reference _askeypad_button_4_blueprint _self))
      (:then_5
        (bind _askeypad_button_5_blueprint (Utilities|Casting|CastToKeypad_Button_5_Blueprint (Variables|/Script/Engine.ChildActorComponent|GetChildActor _array_element)))
        (Variables|/Game/Project_Folder/Blueprints/Keypad_System/Buttons/Keypad_Button_5_Blueprint.Keypad_Button_5_Blueprint_C|SetKeypad%20Actor%20Reference _askeypad_button_5_blueprint _self))
      (:then_6
        (bind _askeypad_button_6_blueprint (Utilities|Casting|CastToKeypad_Button_6_Blueprint (Variables|/Script/Engine.ChildActorComponent|GetChildActor _array_element)))
        (Variables|/Game/Project_Folder/Blueprints/Keypad_System/Buttons/Keypad_Button_6_Blueprint.Keypad_Button_6_Blueprint_C|SetKeypad%20Actor%20Reference _askeypad_button_6_blueprint _self))
      (:then_7
        (bind _askeypad_button_7_blueprint (Utilities|Casting|CastToKeypad_Button_7_Blueprint (Variables|/Script/Engine.ChildActorComponent|GetChildActor _array_element)))
        (Variables|/Game/Project_Folder/Blueprints/Keypad_System/Buttons/Keypad_Button_7_Blueprint.Keypad_Button_7_Blueprint_C|SetKeypad%20Actor%20Reference _askeypad_button_7_blueprint _self))
      (:then_8
        (bind _askeypad_button_8_blueprint (Utilities|Casting|CastToKeypad_Button_8_Blueprint (Variables|/Script/Engine.ChildActorComponent|GetChildActor _array_element)))
        (Variables|/Game/Project_Folder/Blueprints/Keypad_System/Buttons/Keypad_Button_8_Blueprint.Keypad_Button_8_Blueprint_C|SetKeypad%20Actor%20Reference _askeypad_button_8_blueprint _self))
      (:then_9
        (bind _askeypad_button_9_blueprint (Utilities|Casting|CastToKeypad_Button_9_Blueprint (Variables|/Script/Engine.ChildActorComponent|GetChildActor _array_element)))
        (Variables|/Game/Project_Folder/Blueprints/Keypad_System/Buttons/Keypad_Button_9_Blueprint.Keypad_Button_9_Blueprint_C|SetKeypad%20Actor%20Reference _askeypad_button_9_blueprint _self))
      (:then_10
        (bind _askeypad_button_enter_blueprint (Utilities|Casting|CastToKeypad_Button_Enter_Blueprint (Variables|/Script/Engine.ChildActorComponent|GetChildActor _array_element)))
        (Variables|/Game/Project_Folder/Blueprints/Keypad_System/Buttons/Keypad_Button_Enter_Blueprint.Keypad_Button_Enter_Blueprint_C|SetKeypad%20Actor%20Reference _askeypad_button_enter_blueprint _self))
      (:then_11
        (bind _askeypad_button_0_blueprint (Utilities|Casting|CastToKeypad_Button_0_Blueprint (Variables|/Script/Engine.ChildActorComponent|GetChildActor _array_element)))
        (Variables|/Game/Project_Folder/Blueprints/Keypad_System/Buttons/Keypad_Button_0_Blueprint.Keypad_Button_0_Blueprint_C|SetKeypad%20Actor%20Reference _askeypad_button_0_blueprint _self)))))

(fn ConstructionScript)