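; Interactive valve door that the player opens or closes by holding E inside a box trigger, which toggles player input on overlap.
; One timeline drives both the valve's pitch and the door pivot's yaw, pausing when E is released or the player leaves.
; Pressing E reverses the timeline only when the valve track is at full turn, otherwise plays it forward, with a matching 2D open or close sound.
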(event OnComponentBeginOverlap(Box)
  (params (OverlappedComponent :type Primitive%20Component%20Object%20Reference) (OtherActor :type Actor%20Object%20Reference) (OtherComp :type Primitive%20Component%20Object%20Reference) (OtherBodyIndex :type Integer) (bFromSweep :type Boolean) (SweepResult :type Hit%20Result%20Structure%20%28by%20ref%29))
  (Input|EnableInput (Game|GetPlayerController 0)))

(event OnComponentEndOverlap(Box)
  (params (OverlappedComponent :type Primitive%20Component%20Object%20Reference) (OtherActor :type Actor%20Object%20Reference) (OtherComp :type Primitive%20Component%20Object%20Reference) (OtherBodyIndex :type Integer))
  (Input|DisableInput (Game|GetPlayerController 0))
  (Audio|Components|Audio|Stop (Variables|Default|GetSound))
  (bind (_direction _valve _door) (Timeline|Animation Stop)
    (:Update
      (Transformation|SetRelativeRotation (Variables|Default|GetValve) (Math|Rotator|MakeRotator 0.0 _valve 0.0) false false)
      (Transformation|SetRelativeRotation (Variables|Default|GetPivot) (Math|Rotator|MakeRotator 0.0 0.0 _door) false false))
    (:Finished
      (Audio|Components|Audio|Stop (Variables|Default|GetSound)))))

(event Input|KeyboardEvents|E
  (params (Key :type Key%20Structure :default "None"))
  (:Pressed
    (if (>= (stale _valve) 3.6e+02)
      (bind _returnvalue (Audio|SpawnSound2D "/Game/Project_Folder/Sounds/Valve_Close.Valve_Close" 1.0 1.0 0.0 0))
      (Variables|Default|SetSound _returnvalue)
      (bind (_direction _valve _door) (Timeline|Animation Reverse)
        (:Update
          (Transformation|SetRelativeRotation (Variables|Default|GetValve) (Math|Rotator|MakeRotator 0.0 _valve 0.0) false false)
          (Transformation|SetRelativeRotation (Variables|Default|GetPivot) (Math|Rotator|MakeRotator 0.0 0.0 _door) false false))
        (:Finished
          (Audio|Components|Audio|Stop (Variables|Default|GetSound))))
      (else
        (bind _returnvalue_2 (Audio|SpawnSound2D "/Game/Project_Folder/Sounds/Valve_Open.Valve_Open" 1.0 1.0 0.0 0))
        (Variables|Default|SetSound _returnvalue_2)
        (Timeline|Animation Play))))
  (:Released
    (Audio|Components|Audio|Stop (Variables|Default|GetSound))
    (Timeline|Animation Stop)))

(fn ConstructionScript)