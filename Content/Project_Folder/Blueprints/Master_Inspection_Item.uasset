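; Base pickup item that the player can inspect and then add to the inventory or consume.
; On interaction it spawns a far-off Studio actor to present the mesh, name and description, only on first pickup per item class for inventory items.
; It destroys itself once added or when the stubbed PickUpBenefits returns true; UseItem is also a stub.
; Sphere overlap shows an interact widget, and trace focus toggles its border.
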(event OnComponentBeginOverlap(Sphere)
  (params (OverlappedComponent :type Primitive%20Component%20Object%20Reference) (OtherActor :type Actor%20Object%20Reference) (OtherComp :type Primitive%20Component%20Object%20Reference) (OtherBodyIndex :type Integer) (bFromSweep :type Boolean) (SweepResult :type Hit%20Result%20Structure%20%28by%20ref%29))
  (bind _widget (Variables|Default|GetWidget))
  (Utilities|Casting|CastToBP_FirstPersonCharacter OtherActor)
  (bind _returnvalue (UserInterface|CreateWidget "/Game/Project_Folder/Blueprints/Widgets/Interact_Widget.Interact_Widget_C"))
  (bind _output_get (Variables|Default|SetInteraction_Widget _returnvalue))
  (UserInterface|SetWidget _widget _output_get)
  (Rendering|SetVisibility _widget true false))

(event OnComponentEndOverlap(Sphere)
  (params (OverlappedComponent :type Primitive%20Component%20Object%20Reference) (OtherActor :type Actor%20Object%20Reference) (OtherComp :type Primitive%20Component%20Object%20Reference) (OtherBodyIndex :type Integer))
  (Utilities|Casting|CastToBP_FirstPersonCharacter OtherActor)
  (Widget|RemovefromParent (Variables|Default|GetInteraction_Widget))
  (Variables|Default|SetInteraction_Widget 0)
  (Rendering|SetVisibility (Variables|Default|GetWidget) false false))

(event EventBeginPlay
  (Utilities|Struct|SetmembersinItem_Structure (Variables|Default|GetItem%20Structure) (Variables|/Script/Engine.StaticMeshComponent|GetStaticMesh (Variables|Default|GetStaticMesh))))

(event EventCanRecieveTrace
  (params (Can%20Interact :type Boolean))
  (if Can%20Interact
    (bind _interaction_widget (Variables|Default|GetInteraction_Widget)
      (:then
        (Widget|SetRenderOpacity (Variables|/Game/Project_Folder/Blueprints/Widgets/Interact_Widget.Interact_Widget_C|GetInteraction_Border _interaction_widget) 1.0))
      (:else))
    (else
      (bind _interaction_widget_2 (Variables|Default|GetInteraction_Widget)
        (:then
          (Widget|SetRenderOpacity (Variables|/Game/Project_Folder/Blueprints/Widgets/Interact_Widget.Interact_Widget_C|GetInteraction_Border _interaction_widget_2) 0.0))
        (:else)))))

(event EventInteractItems
  (params (Player :type BP%20First%20Person%20Character%20Object%20Reference))
  (bind _item_structure (Variables|Default|GetItem%20Structure))
  (bind _item_structure_2 (Variables|Default|GetItem%20Structure))
  (bind (_itemname _itemdescription) (Utilities|Struct|BreakItem_Structure _item_structure))
  (bind _success (CallFunction|CheckInspect))
  (if _success
    (bind _returnvalue (Game|SpawnActorfromClass "/Game/Project_Folder/Blueprints/Studio.Studio_C" (Math|Transform|MakeTransform "1000000000.000000,0.000000,0.000000") "Undefined" 0 "/Game/Project_Folder/Sounds/Picture_Pickup.Picture_Pickup" 0))
    (Class|InspectInterface|Inspect(Message) _returnvalue Player (Variables|/Script/Engine.StaticMeshComponent|GetStaticMesh (Variables|Default|GetStaticMesh)) _itemname _itemdescription false))
  (if (.canbeadded? _item_structure_2)
    (bind _success_2 (Default|AddtoInventory (Actor|GetComponentbyClass Player "/Game/Project_Folder/Blueprints/Inventory_System/Inventory_Component.Inventory_Component_C") (Utilities|Struct|MakeSlot_Structure (Variables|Default|GetItem%20Structure) 1)))
    (if _success_2
      (Actor|DestroyActor :!label _label))
    (elif (.ispickupbenefitial _item_structure_2)
      (bind _success_3 (CallFunction|PickUpBenefits))
      (if _success_3
        (goto _label)))))

(fn ConstructionScript)

(fn PickUpBenefits
  (return false))

(fn UseItem
  (return false))

(fn CheckInspect
  (bind _item_structure (Variables|Default|GetItem%20Structure))
  (bind _itemclass (Utilities|Struct|BreakItem_Structure _item_structure))
  (if (.canbeadded? (Variables|Default|GetItem%20Structure))
    (bind _asbp_first_person_character (Utilities|Casting|CastToBP_FirstPersonCharacter (Game|GetPlayerCharacter 0)))
    (if (== (Utilities|Array|FindItem (Variables|/Game/Project_Folder/Blueprints/Inventory_System/Inventory_Component.Inventory_Component_C|GetInspected%20Items (Variables|/Game/Project_Folder/BP_FirstPersonCharacter.BP_FirstPersonCharacter_C|GetInventory_Component _asbp_first_person_character)) _itemclass) -1)
      (Utilities|Array|Add (Variables|/Game/Project_Folder/Blueprints/Inventory_System/Inventory_Component.Inventory_Component_C|GetInspected%20Items (Variables|/Game/Project_Folder/BP_FirstPersonCharacter.BP_FirstPersonCharacter_C|GetInventory_Component _asbp_first_person_character)) _itemclass)
      (return true)
      (else
        (return false)))
    (else
      (return true))))