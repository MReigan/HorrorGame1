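; Pills is an inspection item Blueprint with pick-up and use functions, both of which return true on success.
; Pick Up Benefits casts the player character to BP_FirstPersonCharacter and adds two slots to its InventoryComponent.
; Use Item is only a placeholder that prints a "Bandage Used" message, with no healing or other effect.
; The event graph and construction script add no logic of their own.
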(event EventBeginPlay
  (|CallParentFunction) ; This node is disabled and will not be called.\nDrag off pins to build functionality.
)

(event Collision|EventActorBeginOverlap
  (params (OtherActor :type Actor%20Object%20Reference))
  (|CallParentFunction OtherActor) ; This node is disabled and will not be called.\nDrag off pins to build functionality.
)

(event EventTick
  (params (DeltaSeconds :type Float%20%28single-precision%29))
  (|CallParentFunction DeltaSeconds) ; This node is disabled and will not be called.\nDrag off pins to build functionality.
)

(fn ConstructionScript
  (|CallParentFunction))

(fn PickUpBenefits
  (bind _asbp_first_person_character (Utilities|Casting|CastToBP_FirstPersonCharacter (Game|GetPlayerCharacter 0)))
  (Variables|/Game/Project_Folder/Blueprints/Inventory_System/Inventory_Component.Inventory_Component_C|SetNumber%20Of%20Slots (Variables|/Game/Project_Folder/BP_FirstPersonCharacter.BP_FirstPersonCharacter_C|GetInventory_Component _asbp_first_person_character) (+ (Variables|/Game/Project_Folder/Blueprints/Inventory_System/Inventory_Component.Inventory_Component_C|GetNumber%20Of%20Slots (Variables|/Game/Project_Folder/BP_FirstPersonCharacter.BP_FirstPersonCharacter_C|GetInventory_Component _asbp_first_person_character)) 2))
  (return true))

(fn UseItem
  (Development|PrintString "Bandage Used")
  (return true))