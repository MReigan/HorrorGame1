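; Interactive Resident Evil-style door that cycles through closed, partially open and open states on each player interaction, with a matching sound per step.
; A DoOnce locks input while Tick eases the door yaw toward its target with FInterpTo, until a short timer advances the state and resets the lock.
; A dot product makes it swing according to the player's facing.
; A box overlap toggles the widget for the first-person character.
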(event OnComponentEndOverlap(Box)
  (params (OverlappedComponent :type Primitive%20Component%20Object%20Reference) (OtherActor :type Actor%20Object%20Reference) (OtherComp :type Primitive%20Component%20Object%20Reference) (OtherBodyIndex :type Integer))
  (Utilities|Casting|CastToBP_FirstPersonCharacter OtherActor)
  (Development|SetHiddeninGame (Variables|Default|GetWidget) true false))

(event OnComponentBeginOverlap(Box)
  (params (OverlappedComponent :type Primitive%20Component%20Object%20Reference) (OtherActor :type Actor%20Object%20Reference) (OtherComp :type Primitive%20Component%20Object%20Reference) (OtherBodyIndex :type Integer) (bFromSweep :type Boolean) (SweepResult :type Hit%20Result%20Structure%20%28by%20ref%29))
  (Utilities|Casting|CastToBP_FirstPersonCharacter OtherActor)
  (Development|SetHiddeninGame (Variables|Default|GetWidget) false false))

(event Custom|Manage_Door
  (switch Utilities|FlowControl|Switch|SwitchonDoor_States (Variables|Default|GetDoor_State)
    (:NewEnumerator0
      (CallFunction|RotateDoor (* 2e+01 (Variables|Default|GetDoor%20Side%20To%20Open))))
    (:NewEnumerator1
      (CallFunction|RotateDoor (* 9e+01 (Variables|Default|GetDoor%20Side%20To%20Open))))
    (:NewEnumerator2
      (CallFunction|RotateDoor 0.0))))

(event Custom|Interacting%20With%20Door
  (params (Player :type BP%20First%20Person%20Character%20Object%20Reference))
  (bind _returnvalue (Transformation|GetActorForwardVector Player))
  (bind _door_base (Variables|Default|GetDoor_Base))
  (bind _returnvalue_2 (Math|Vector|GetForwardVector _door_base))
  (bind _returnvalue_3 (Math|Vector|DotProduct _returnvalue _returnvalue_2))
  (Utilities|FlowControl|DoOnce false
    (:Completed
      (CallFunction|PlayDoorSound)
      (Development|PrintString (Utilities|String|ToString(Float) _returnvalue_3))
      (if (> _returnvalue_3 0.0)
        (Variables|Default|SetDoor%20Side%20To%20Open 1.0)
        (else
          (Variables|Default|SetDoor%20Side%20To%20Open -1.0)))
      (Variables|Default|SetIs%20Interacting true)
      (Utilities|Time|SetTimerbyEvent (delegate Custom|Stop%20Interacting%20With%20Door) 0.67))))

(event Custom|Rotate%20Door
  (params (Rotation%20To%20Set :type Float%20%28double-precision%29))
  (Transformation|SetRelativeRotation (Variables|Default|GetDoor_Base) (Math|Rotator|MakeRotator 0.0 0.0 (Math|Interpolation|FInterpTo (.Yaw (Math|Rotator|BreakRotator (Variables|/Script/Engine.SceneComponent|GetRelativeRotation (Variables|Default|GetDoor_Base)))) Rotation%20To%20Set (Utilities|Time|GetWorldDeltaSeconds) 5.0)) false false))

(event Custom|Stop%20Interacting%20With%20Door
  (Variables|Default|SetIs%20Interacting false)
  (Utilities|FlowControl|Sequence
    (:then_0
      (Utilities|FlowControl|DoOnce false) ; enters at Reset
    )
    (:then_1
      (switch Utilities|FlowControl|Switch|SwitchonDoor_States (Variables|Default|GetDoor_State)
        (:NewEnumerator0
          (bind _output_get (Variables|Default|SetDoor_State "NewEnumerator1"))
          (Development|PrintString (Utilities|String|EnumtoString _output_get)))
        (:NewEnumerator1
          (bind _output_get_2 (Variables|Default|SetDoor_State "NewEnumerator2"))
          (Development|PrintString (Utilities|String|EnumtoString _output_get_2)))
        (:NewEnumerator2
          (bind _output_get_3 (Variables|Default|SetDoor_State "NewEnumerator0"))
          (Development|PrintString (Utilities|String|EnumtoString _output_get_3)))))))

(event Custom|Play%20Door%20Sound
  (bind _returnvalue (Transformation|GetActorLocation))
  (switch Utilities|FlowControl|Switch|SwitchonDoor_States (Variables|Default|GetDoor_State)
    (:NewEnumerator0
      (Audio|PlaySoundatLocation "/Game/Project_Folder/Sounds/Other/Wooden_Crack_4.Wooden_Crack_4" _returnvalue "0, 0, 0" 1.0 1.0 0.0 0 0 0 0))
    (:NewEnumerator1
      (Audio|PlaySoundatLocation "/Game/Project_Folder/Sounds/Door_Open.Door_Open" _returnvalue "0, 0, 0" 1.0 1.0 0.0 0 0 0 0))
    (:NewEnumerator2
      (Audio|PlaySoundatLocation "/Game/Project_Folder/Sounds/Door_Close.Door_Close" _returnvalue "0, 0, 0" 1.0 1.0 0.0 0 0 0 0))))

(event EventTick
  (params (DeltaSeconds :type Float%20%28single-precision%29))
  (if (Variables|Default|GetIs%20Interacting)
    (CallFunction|ManageDoor)))

(fn ConstructionScript)