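; Hinged door Blueprint that swings open on OnSuccess and has an Interact toggle for opening and closing.
; OnSuccess and Interact's open branch share a timeline that lerps DoorBase yaw through a quarter turn, with positional open sound.
; Closing reverses the timeline with its own sound.
; Interact only acts while IsDoorMoving is true, a flag cleared when the timeline finishes; IsFinished is set during timeline updates.
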(event EventOnSuccess
  (Audio|PlaySoundatLocation "/Game/Project_Folder/Sounds/Door_Open.Door_Open" (Transformation|GetWorldLocation (Variables|Default|GetDoor_Base)) "0, 0, 0" 1.0 1.0 0.0 0 0 0 0)
  (bind _door_alpha (Timeline|Door_Timeline Play)
    (:Update
      (Transformation|SetRelativeRotation (Variables|Default|GetDoor_Base) (Math|Rotator|MakeRotator 0.0 0.0 (Math|Float|Lerp 0.0 -9e+01 _door_alpha)) false false)
      (Variables|Default|SetIs%20Finished? true))
    (:Finished
      (Variables|Default|SetIs%20Door%20Moving? false))))

(event EventInteract
  (bind _door_base (Variables|Default|GetDoor_Base))
  (bind _returnvalue (Transformation|GetWorldLocation _door_base))
  (if (not (not (Variables|Default|GetIs%20Door%20Moving?)))
    (Variables|Default|SetIs%20Door%20Moving? true)
    (bind _output_get (Variables|Default|SetOpening (not (Variables|Default|GetOpening))))
    (if _output_get
      (Audio|PlaySoundatLocation "/Game/Project_Folder/Sounds/Door_Open.Door_Open" _returnvalue "0, 0, 0" 1.0 1.0 0.0 0 0 0 0)
      (bind _door_alpha (Timeline|Door_Timeline Play)
        (:Update
          (Transformation|SetRelativeRotation (Variables|Default|GetDoor_Base) (Math|Rotator|MakeRotator 0.0 0.0 (Math|Float|Lerp 0.0 -9e+01 _door_alpha)) false false)
          (Variables|Default|SetIs%20Finished? true))
        (:Finished
          (Variables|Default|SetIs%20Door%20Moving? false)))
      (else
        (Audio|PlaySoundatLocation "/Game/Project_Folder/Sounds/Door_Close.Door_Close" _returnvalue "0, 0, 0" 1.0 1.0 0.0 0 0 0 0)
        (Timeline|Door_Timeline Reverse)))))

(fn ConstructionScript)